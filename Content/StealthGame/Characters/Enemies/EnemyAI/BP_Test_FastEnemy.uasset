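; Test fast stealth-game enemy that patrols, investigates noises and sprints after the player, all in Blueprint without a behavior tree.
; Tick uses CanMove and PlayerVisible to pick chase or patrol (target points or random) via AIMoveTo, changing speed and spotlight color.
; PawnSensing drives noise investigation and sight, which expires through a retriggerable delay; first chase triggers a bark.
; Reaching the player plays an attack montage whose notify sphere-traces from the hand, reloading the checkpoint on hit.
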(event `self.ReceiveTick`
  (params (DeltaSeconds :type "Float (single-precision)"))
  (bind _bplayervisible (`self.bPlayerVisible`))
  (bind _returnvalue (`SceneComponent.K2_GetComponentLocation` (`self.CapsuleComponent`)))
  (bind _returnvalue_2 (`SceneComponent.K2_GetComponentLocation` (`self.CapsuleComponent`)))
  ; Check if Movement is Possible and if Player Can Be Chased
  (if (`self.bCanMove`)
    (if _bplayervisible
      (if (`self.bChasing`)
        (`self.Chase Player`)
        (else
          (`PawnNoiseEmitterComponent.MakeNoise` (`self.PawnNoiseEmitter`) self 0.0 _returnvalue)
          (`GameplayStatics.PlaySoundAtLocation` "/Game/Developer/Audio/260776__deleted_user_3424813__angry-dog-bark-snarl-flat.260776__deleted_user_3424813__angry-dog-bark-snarl-flat" _returnvalue (struct) 1.0 1.0 0.0 null null null null)
          (`self.Chase Player`)))
      (elif (`self.bTargetPointMovement`)
        (`self.MovetoCustomPatrolPoint`)
        (else
          (`self.Patrol Random`))))
    (elif _bplayervisible
      (if (`self.bChasing`)
        (`self.Chase Player`)
        (else
          (`PawnNoiseEmitterComponent.MakeNoise` (`self.PawnNoiseEmitter`) self 0.0 _returnvalue_2)
          (`GameplayStatics.PlaySoundAtLocation` "/Game/Developer/Audio/260776__deleted_user_3424813__angry-dog-bark-snarl-flat.260776__deleted_user_3424813__angry-dog-bark-snarl-flat" _returnvalue_2 (struct) 1.0 1.0 0.0 null null null null)
          (`self.Chase Player`))))))

(event `Attack`
  (bind _returnvalue (`SceneComponent.GetSocketLocation` (`self.Mesh`) "hand_r"))
  ;[0.15 0.1407 0.04319 0.5] Bonk
  (`/Engine/EditorBlueprintResources/StandardMacros.DoOnce` false :!label _label ; Only Reset Attack on miss.
    (:`Completed`
      (bind _notifyname (`|PlayMontage` (`self.Mesh`) "/Game/StealthGame/Characters/Enemies/EnemyAI/AM_Attack_01.AM_Attack_01") ; Play the AM_Attack_01
        (:`OnCompleted`
          (`self.ResetAttack`))
        (:`OnNotifyBegin`
          (switch `name` _notifyname ; Pick the proper attack type(standard when there is more than one type of attack)
            (:`AttackDamage`
              (bind (_outhits _returnvalue_2) (`KismetSystemLibrary.SphereTraceMultiForObjects` _returnvalue (+ _returnvalue (* (`self.GetActorForwardVector`) (`self.MeleeTraceDistance`))) (`self.MeleeTraceRadius`) (`|MakeArray` "ObjectTypeQuery3" :!type "EObjectTypeQuery Enum"))) ; Trace forward from hand socket.
              (if _returnvalue_2
                (for _array_element _outhits
                  (bind _asbp_third_person_character_custom (cast `/Game/StealthGame/Core/Characters/PlayerCharacter/BP_ThirdPersonCharacterCustom` (`.HitActor` (`GameplayStatics.BreakHitResult` _array_element))))
                  (`/Game/StealthGame/Core/Characters/PlayerCharacter/BP_ThirdPersonCharacterCustom.LoadCheckpoint` _asbp_third_person_character_custom))))))))))

(event `ResetAttack`
  ;[0.15 0.1407 0.04319 0.5] Bonk
  (goto _label :!via `Reset`))

(event `self.PawnSensing.OnHearNoise`
  (params (Instigator :type "Pawn Object Reference") (Location :type "Vector Structure (by ref)") (Volume :type "Float (single-precision)"))
  ; Pawn Sensing
  (set `self.bCanMove` false)
  (`|AIMoveTo` self Location Instigator 50.0
    (:`OnSuccess`
      _)
    (:`OnFail`
      _))
  (`KismetSystemLibrary.Delay` 5.0)
  (set `self.bCanMove` true))

(event `self.PawnSensing.OnSeePawn`
  (params (Pawn :type "Pawn Object Reference"))
  ; Pawn Sensing
  (`|ExecutionSequence`
    (:`then_0`
      (cast `/Game/StealthGame/Core/Characters/PlayerCharacter/BP_ThirdPersonCharacterCustom` Pawn
        (:`then`
          (set `self.bPlayerVisible` true))
        (:`CastFailed`
          (set `self.bPlayerVisible` false))))
    (:`then_1`
      (`KismetSystemLibrary.RetriggerableDelay` 3.0)
      (set `self.bPlayerVisible` false))))

(event `Chase Player`
  ; Chase Player
  (set `self.bChasing` true)
  (`LightComponent.SetLightColor` (`self.SpotLight`) (struct :`R` 0.745999 :`A` 1.0) true)
  (`self.UpdateWalkSpeed` 700.0)
  (set `self.bCanMove` false)
  (`|AIMoveTo` self (0.0 0.0 0.0) (`GameplayStatics.GetPlayerCharacter` 0) 50.0
    (:`OnSuccess`
      (`self.Attack`)
      (`KismetSystemLibrary.Delay` 3.0)
      (set `self.bCanMove` true))
    (:`OnFail`
      (`KismetSystemLibrary.Delay` 5.0)
      (set `self.bCanMove` true))))

(event `Patrol Random`
  ; Patrol Random
  (`LightComponent.SetLightColor` (`self.SpotLight`) (struct :`R` 1.0 :`G` 1.0 :`B` 1.0 :`A` 1.0) true)
  (`self.UpdateWalkSpeed` 1.0)
  (set `self.bCanMove` false)
  (`|AIMoveTo` self (`NavigationSystemV1.K2_GetRandomReachablePointInRadius` (`self.K2_GetActorLocation`) 2000.0 null null) null 50.0
    (:`OnSuccess`
      _)
    (:`OnFail`
      _))
  (`KismetSystemLibrary.Delay` 3.0)
  (set `self.bCanMove` true))

(event `MovetoCustomPatrolPoint`
  ; Patrol to Points
  (`LightComponent.SetLightColor` (`self.SpotLight`) (struct :`R` 1.0 :`G` 1.0 :`B` 1.0 :`A` 1.0) true)
  (`self.UpdateWalkSpeed` 300.0)
  (set `self.bCanMove` false)
  (`|AIMoveTo` self (0.0 0.0 0.0) (`|GetArrayItem` (`self.PatrolTargetPoints`) (`self.PatrolTargetPointIndex`)) 50.0
    (:`OnSuccess`
      (`KismetSystemLibrary.Delay` 0.3)
      (set `self.bCanMove` true)
      (`self.SetNextPatrolPointIndex`))))

(event `SetNextPatrolPointIndex`
  ; Set Next Patrol Point Index
  (set `self.PatrolTargetPointIndex` (mod (+ (`self.PatrolTargetPointIndex`) 1) (`KismetArrayLibrary.Array_Length` (`self.PatrolTargetPoints`)))))

(fn `UpdateWalkSpeed`
  (params (NewWalkSpeed :type "Float (double-precision)"))
  (set `CharacterMovementComponent.MaxWalkSpeed` NewWalkSpeed (`self.CharacterMovement`)))

(fn `UserConstructionScript`)